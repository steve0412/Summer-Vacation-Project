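; Grunt is a Blueprint for an attacking actor that deals fixed point damage to whatever overlaps its AttackCollision component.
; The damage passes the actor's forward vector as hit direction, the sweep result as hit info, and its controller as instigator.
; OnAttackBegin and OnAttackEnd are empty, so this graph never toggles the collision.
; A forward sphere trace with debug drawing is left unconnected and never runs.
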(event OnComponentBeginOverlap(AttackCollision)
  (params (OverlappedComponent :type Primitive%20Component%20Object%20Reference) (OtherActor :type Actor%20Object%20Reference) (OtherComp :type Primitive%20Component%20Object%20Reference) (OtherBodyIndex :type Integer) (bFromSweep :type Boolean) (SweepResult :type Hit%20Result%20Structure%20%28by%20ref%29))
  (Game|Damage|ApplyPointDamage OtherActor 5e+01 (Transformation|GetActorForwardVector) SweepResult (Pawn|GetController) self))

(event Custom|OnAttackBegin)

(event Custom|OnAttackEnd)

(event Collision|EventActorBeginOverlap
  (params (OtherActor :type Actor%20Object%20Reference)))

(event EventBeginPlay)

(event EventTick
  (params (DeltaSeconds :type Float%20%28single-precision%29)))

(fn ConstructionScript
  (|CallParentFunction))