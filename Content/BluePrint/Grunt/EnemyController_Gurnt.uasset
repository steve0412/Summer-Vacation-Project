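; AI controller for the Grunt enemy that starts its behavior tree when it possesses a pawn.
; On possession it sets up the Grunt blackboard with the pawn's spawn location as home, a default idle time and a random navigable point near home as the first target location.
; It then runs the Grunt behavior tree, which takes over from those seeded keys.
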(event EventOnPossess
  (params (PossessedPawn :type Pawn%20Object%20Reference))
  (bind _returnvalue (Pawn|GetControlledPawn))
  (bind _returnvalue_2 (Transformation|GetActorLocation _returnvalue))
  (Utilities|FlowControl|Sequence
    (:then_0
      (Class|AIController|UseBlackboard "/Game/BluePrint/Grunt/EnemyBB_Grunt.EnemyBB_Grunt")
      (AI|Components|Blackboard|SetValueasVector (Variables|Default|GetBlackboard) (Variables|Default|GetHome%20Loc%20Key) _returnvalue_2)
      (AI|Components|Blackboard|SetValueasFloat (Variables|Default|GetBlackboard) (Variables|Default|GetIdle%20Time%20Key) 3.0)
      (AI|Components|Blackboard|SetValueasVector (Variables|Default|GetBlackboard) (Variables|Default|GetTarget%20Loc%20Key) (.RandomLocation (Class|NavigationSystem|GetRandomPointinNavigableRadius _returnvalue_2 5e+02))))
    (:then_1
      (AI|RunBehaviorTree "/Game/BluePrint/Grunt/EnemyBT_Grunt.EnemyBT_Grunt"))))

(fn ConstructionScript)