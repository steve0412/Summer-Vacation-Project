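; Behavior tree decorator that checks whether the Grunt enemy has a target to aggro on.
; Each check writes the controlled pawn's Instigator into the Target blackboard key and passes if that actor is valid.
; On failure it sets the Enemy_Grunt to the first value of its state enum, so the condition also changes blackboard and pawn state.
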(fn PerformConditionCheck
  (params (OwnerActor :type Actor%20Object%20Reference))
  (bind _returnvalue (AI|GetAIController OwnerActor))
  (Class|BTFunctionLibrary|SetBlackboardValueasObject (Variables|Default|GetTarget) (Variables|/Script/Engine.Actor|GetInstigator (Pawn|GetControlledPawn _returnvalue)))
  (Utilities|IsValid (AI|BehaviorTree|GetBlackboardValueasActor (Variables|Default|GetTarget))
    (:Is%20Valid
      (return true))
    (:Is%20Not%20Valid
      (bind _asenemy_grunt (Utilities|Casting|CastToEnemy_Grunt (Pawn|GetControlledPawn _returnvalue))
        (:then
          (Default|SetState _asenemy_grunt "NewEnumerator0")
          (return false))
        (:CastFailed
          (return false))))))