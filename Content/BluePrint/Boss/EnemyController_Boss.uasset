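; EnemyController_Boss is the AI controller for the boss enemy.
; On possess, it applies the EnemyBB_Boss blackboard and then runs the EnemyBT_Boss behavior tree, which is left to drive the boss.
; Disconnected nodes that would seed home location, idle time and a random navigable target location in the blackboard never run, so this controller sets no key values.
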(event EventOnPossess
  (params (PossessedPawn :type Pawn%20Object%20Reference))
  (Utilities|FlowControl|Sequence
    (:then_0
      (Class|AIController|UseBlackboard "/Game/BluePrint/Boss/EnemyBB_Boss.EnemyBB_Boss"))
    (:then_1
      (AI|RunBehaviorTree "/Game/BluePrint/Boss/EnemyBT_Boss.EnemyBT_Boss"))))

(fn ConstructionScript)