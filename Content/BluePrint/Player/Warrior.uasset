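; Warrior player pawn Blueprint that handles basic movement and camera-look input through axis mappings.
; MoveForward and MoveRight add movement input relative to control rotation, with forward using only yaw and right using the full rotation.
; Turn and LookUp pass their axis values to controller yaw and pitch input.
; The construction script is empty, and the event graph holds no other gameplay logic.
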(event Input|AxisEvents|InputAxisTurn
  (params (AxisValue :type Float%20%28single-precision%29))
  (Pawn|Input|AddControllerYawInput AxisValue))

(event Input|AxisEvents|InputAxisMoveForward
  (params (AxisValue :type Float%20%28single-precision%29))
  (Pawn|Input|AddMovementInput (Math|Vector|GetForwardVector (Math|Rotator|MakeRotator 0.0 0.0 (.yaw (Pawn|GetControlRotation :!class /Script/Engine.Pawn)))) AxisValue false))

(event Input|AxisEvents|InputAxisLookUp
  (params (AxisValue :type Float%20%28single-precision%29))
  (Pawn|Input|AddControllerPitchInput AxisValue))

(event Input|AxisEvents|InputAxisMoveRight
  (params (AxisValue :type Float%20%28single-precision%29))
  (Pawn|Input|AddMovementInput (Math|Vector|GetRightVector (Pawn|GetControlRotation :!class /Script/Engine.Pawn)) AxisValue false))

(fn ConstructionScript)