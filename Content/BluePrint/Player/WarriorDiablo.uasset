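; WarriorDiablo is a player character Blueprint with camera-relative movement, jumping, a ranged attack and health, driven by a pawn state enum.
; In PEACE, Tick turns movement input plus camera yaw into control rotation and moves the character forward.
; Fire switches the state to BATTLE, and the OnAttackHit event spawns a Ball at the character's transform.
; Damage reduces HP, and depletion sets DEAD and shows the GameOverBlack widget.
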(event Custom|OnAttackHit
  (Game|SpawnActorfromClass "/Game/BluePrint/Ball.Ball_C" (Transformation|GetActorTransform) "Undefined" 0 0))

(event EventBeginPlay
  (Variables|Default|SetCurrentHP (Variables|Default|GetMaxHP)))

(event EventTick
  (params (DeltaSeconds :type Float%20%28single-precision%29))
  (switch Utilities|FlowControl|Switch|SwitchonPlayerState (Variables|Default|GetCurrentStatePawn)
    (:NewEnumerator0
      (if (|입력이들어왔는가?)
        (Pawn|SetControlRotation (Pawn|GetController) (Math|Rotator|MakeRotator 0.0 0.0 (.yaw (Math|Rotator|CombineRotators (Math|Rotator|MakeRotfromX (Math|Vector|MakeVector (Input|AxisValues|GetMoveForward) (Input|AxisValues|GetMoveRight) 0.0)) (Camera|GetCameraRotation (Game|GetPlayerCameraManager 0))))))
        (Pawn|Input|AddMovementInput (Transformation|GetActorForwardVector) 1.0 false)))))

(event Game|Damage|EventAnyDamage
  (params (Damage :type Float%20%28single-precision%29) (DamageType :type Damage%20Type%20Object%20Reference) (InstigatedBy :type Controller%20Object%20Reference) (DamageCauser :type Actor%20Object%20Reference))
  (bind _output_get (Variables|Default|SetCurrentHP (- (Variables|Default|GetCurrentHP) Damage)))
  (if (> _output_get 0.0)
    (Development|PrintString (Utilities|String|ToString(Float) (Variables|Default|GetCurrentHP)))
    (else
      (Variables|Default|SetCurrentStatePawn "NewEnumerator2")
      (bind _returnvalue (UserInterface|CreateWidget "/Game/BluePrint/HUD/GameOverBlack.GameOverBlack_C"))
      (UserInterface|Viewport|AddtoPlayerScreen _returnvalue))))

(event Input|ActionEvents|InputActionFire
  (params (Key :type Key%20Structure))
  (:Pressed
    (Variables|Default|SetCurrentStatePawn "NewEnumerator1")))

(event Input|ActionEvents|InputActionJump
  (params (Key :type Key%20Structure))
  (:Pressed
    (Character|Jump)))

(fn ConstructionScript)