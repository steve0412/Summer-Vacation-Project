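; EnemyController is the AI controller for a bear enemy, setting up its Blackboard and Behavior Tree when it possesses a pawn.
; On possession it uses EnemyBB, storing the pawn's location as home, a fixed idle time, and a random navigable point near the pawn as the first target.
; It then runs EnemyBT, which receives these seeded values.
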(event EventOnPossess
  (params (PossessedPawn :type Pawn%20Object%20Reference))
  (bind _returnvalue (Pawn|GetControlledPawn))
  (bind _returnvalue_2 (Transformation|GetActorLocation _returnvalue))
  (Utilities|FlowControl|Sequence
    (:then_0
      (Class|AIController|UseBlackboard "/Game/BluePrint/Bear/EnemyBB.EnemyBB")
      (AI|Components|Blackboard|SetValueasVector (Variables|Default|GetBlackboard) (Variables|Default|GetHome%20Loc%20Key) _returnvalue_2)
      (AI|Components|Blackboard|SetValueasFloat (Variables|Default|GetBlackboard) (Variables|Default|GetIdle%20Time%20Key) 5.0)
      (AI|Components|Blackboard|SetValueasVector (Variables|Default|GetBlackboard) (Variables|Default|GetTarget%20Loc%20Key) (.RandomLocation (Class|NavigationSystem|GetRandomPointinNavigableRadius _returnvalue_2 1e+03))))
    (:then_1
      (AI|RunBehaviorTree "/Game/BluePrint/Bear/EnemyBT.EnemyBT"))))

(fn ConstructionScript)