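; Bear pawn with a melee attack that damages actors touching its Box hitbox.
; The box starts without collision, and OnAttackBegin and OnAttackEnd switch it between query-only and off, limiting hits to the attack window.
; Each overlap applies fixed point damage along the bear's forward vector, crediting its controller as instigator.
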(event OnComponentBeginOverlap(Box)
  (params (OverlappedComponent :type Primitive%20Component%20Object%20Reference) (OtherActor :type Actor%20Object%20Reference) (OtherComp :type Primitive%20Component%20Object%20Reference) (OtherBodyIndex :type Integer) (bFromSweep :type Boolean) (SweepResult :type Hit%20Result%20Structure%20%28by%20ref%29))
  (Game|Damage|ApplyPointDamage OtherActor 3e+01 (Transformation|GetActorForwardVector) SweepResult (Pawn|GetController) self))

(event Custom|OnAttackBegin
  (Collision|SetCollisionEnabled (Variables|Default|GetBox) "QueryOnly"))

(event Custom|OnAttackEnd
  (Collision|SetCollisionEnabled (Variables|Default|GetBox) "NoCollision"))

(event EventBeginPlay
  (Collision|SetCollisionEnabled (Variables|Default|GetBox) "NoCollision"))

(fn ConstructionScript
  (|CallParentFunction))